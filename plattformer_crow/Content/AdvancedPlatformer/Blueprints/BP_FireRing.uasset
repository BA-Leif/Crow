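; BP_FireRing is a fire ring hazard that damages the side-scroller player on contact.
; Four box collision components each handle begin overlap with identical, duplicated logic: cast to BP_SideScrollerCharacterAdvanced, then subtract a fixed amount directly from its Health.
; Each hit prints the new Health to screen; the damage system, death handling and any cooldown are absent here, so every box entered deals damage separately.
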(event `self.Box.OnComponentBeginOverlap`
  (params (OverlappedComponent :type "PrimitiveComponent Object Reference") (OtherActor :type "Actor Object Reference") (OtherComp :type "PrimitiveComponent Object Reference") (OtherBodyIndex :type Integer) (bFromSweep :type Boolean) (SweepResult :type "HitResult Structure (by ref)"))
  ;[1 1 1] When player overlap box collision this will damage him
  (bind _asbp_side_scroller_character_advanced (cast `/Game/AdvancedPlatformer/Blueprints/BP_SideScrollerCharacterAdvanced` OtherActor))
  (bind _output_get (set `/Game/AdvancedPlatformer/Blueprints/BP_SideScrollerCharacterAdvanced.Health` (- (`/Game/AdvancedPlatformer/Blueprints/BP_SideScrollerCharacterAdvanced.Health` _asbp_side_scroller_character_advanced) 20.0) _asbp_side_scroller_character_advanced))
  (`KismetSystemLibrary.PrintString` (`KismetStringLibrary.Conv_DoubleToString` _output_get)))

(event `self.Box1.OnComponentBeginOverlap`
  (params (OverlappedComponent :type "PrimitiveComponent Object Reference") (OtherActor :type "Actor Object Reference") (OtherComp :type "PrimitiveComponent Object Reference") (OtherBodyIndex :type Integer) (bFromSweep :type Boolean) (SweepResult :type "HitResult Structure (by ref)"))
  ;[1 1 1] When player overlap box collision this will damage him
  (bind _asbp_side_scroller_character_advanced (cast `/Game/AdvancedPlatformer/Blueprints/BP_SideScrollerCharacterAdvanced` OtherActor))
  (bind _output_get (set `/Game/AdvancedPlatformer/Blueprints/BP_SideScrollerCharacterAdvanced.Health` (- (`/Game/AdvancedPlatformer/Blueprints/BP_SideScrollerCharacterAdvanced.Health` _asbp_side_scroller_character_advanced) 20.0) _asbp_side_scroller_character_advanced))
  (`KismetSystemLibrary.PrintString` (`KismetStringLibrary.Conv_DoubleToString` _output_get)))

(event `self.Box2.OnComponentBeginOverlap`
  (params (OverlappedComponent :type "PrimitiveComponent Object Reference") (OtherActor :type "Actor Object Reference") (OtherComp :type "PrimitiveComponent Object Reference") (OtherBodyIndex :type Integer) (bFromSweep :type Boolean) (SweepResult :type "HitResult Structure (by ref)"))
  ;[1 1 1] When player overlap box collision this will damage him
  (bind _asbp_side_scroller_character_advanced (cast `/Game/AdvancedPlatformer/Blueprints/BP_SideScrollerCharacterAdvanced` OtherActor))
  (bind _output_get (set `/Game/AdvancedPlatformer/Blueprints/BP_SideScrollerCharacterAdvanced.Health` (- (`/Game/AdvancedPlatformer/Blueprints/BP_SideScrollerCharacterAdvanced.Health` _asbp_side_scroller_character_advanced) 20.0) _asbp_side_scroller_character_advanced))
  (`KismetSystemLibrary.PrintString` (`KismetStringLibrary.Conv_DoubleToString` _output_get)))

(event `self.Box3.OnComponentBeginOverlap`
  (params (OverlappedComponent :type "PrimitiveComponent Object Reference") (OtherActor :type "Actor Object Reference") (OtherComp :type "PrimitiveComponent Object Reference") (OtherBodyIndex :type Integer) (bFromSweep :type Boolean) (SweepResult :type "HitResult Structure (by ref)"))
  ;[1 1 1] When player overlap box collision this will damage him
  (bind _asbp_side_scroller_character_advanced (cast `/Game/AdvancedPlatformer/Blueprints/BP_SideScrollerCharacterAdvanced` OtherActor))
  (bind _output_get (set `/Game/AdvancedPlatformer/Blueprints/BP_SideScrollerCharacterAdvanced.Health` (- (`/Game/AdvancedPlatformer/Blueprints/BP_SideScrollerCharacterAdvanced.Health` _asbp_side_scroller_character_advanced) 20.0) _asbp_side_scroller_character_advanced))
  (`KismetSystemLibrary.PrintString` (`KismetStringLibrary.Conv_DoubleToString` _output_get)))

(fn `UserConstructionScript`)