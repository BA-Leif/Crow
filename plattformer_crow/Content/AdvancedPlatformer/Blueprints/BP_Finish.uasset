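; BP_Finish is the level finish trigger for the advanced side-scroller platformer.
; When a BP_SideScrollerCharacterAdvanced overlaps its Box, a DoOnce gate runs the finish sequence a single time.
; It shows the finish widget, plays the character's applause audio, then adds the final score widget to the viewport.
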(event `self.Box.OnComponentBeginOverlap`
  (params (OverlappedComponent :type "PrimitiveComponent Object Reference") (OtherActor :type "Actor Object Reference") (OtherComp :type "PrimitiveComponent Object Reference") (OtherBodyIndex :type Integer) (bFromSweep :type Boolean) (SweepResult :type "HitResult Structure (by ref)"))
  ;[1 1 1] EventFinishLevel
  (bind _asbp_side_scroller_character_advanced (cast `/Game/AdvancedPlatformer/Blueprints/BP_SideScrollerCharacterAdvanced` OtherActor))
  (set `self.Character` _asbp_side_scroller_character_advanced)
  (`/Engine/EditorBlueprintResources/StandardMacros.DoOnce` false
    (:`Completed`
      (bind _returnvalue (`|CreateWidget` "/Game/AdvancedPlatformer/Widgets/BP_Finish_Widget.BP_Finish_Widget_C"))
      (`UserWidget.AddToViewport` _returnvalue 0)
      (`AudioComponent.Play` (`/Game/AdvancedPlatformer/Blueprints/BP_SideScrollerCharacterAdvanced.Applause_Wav` (`self.Character`)) 0.0)
      (cast `/Game/AdvancedPlatformer/Blueprints/BP_SideScrollerCharacterAdvanced` (`GameplayStatics.GetPlayerCharacter` 0))
      (bind _returnvalue_2 (`|CreateWidget` "/Game/AdvancedPlatformer/Widgets/BP_FinalScore_Widget.BP_FinalScore_Widget_C"))
      (`UserWidget.AddToViewport` _returnvalue_2 0))))

(fn `UserConstructionScript`)