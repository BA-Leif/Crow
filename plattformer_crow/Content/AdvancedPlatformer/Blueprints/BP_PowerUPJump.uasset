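; BP_PowerUPJump is a rotating pickup that enables the power-up jump on the advanced side-scroller character.
; Box overlap casts to the character and calls its ResetPowerUpJump, then a DoOnce gate sets its PowerUPJump flag.
; That gated step also prints a message, removes the cube, plays the character's power-up sound and shows a widget.
; The actor destroys itself after a short delay.
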(event `self.ReceiveBeginPlay`
  ;[1 1 1] RotatingEvent
  (`AddComponent|NODE_AddRotatingMovementComponent-0`))

(event `self.Box.OnComponentBeginOverlap`
  (params (OverlappedComponent :type "PrimitiveComponent Object Reference") (OtherActor :type "Actor Object Reference") (OtherComp :type "PrimitiveComponent Object Reference") (OtherBodyIndex :type Integer) (bFromSweep :type Boolean) (SweepResult :type "HitResult Structure (by ref)"))
  ;[1 1 1] PowerUpJumpEvent
  (bind _asbp_side_scroller_character_advanced (cast `/Game/AdvancedPlatformer/Blueprints/BP_SideScrollerCharacterAdvanced` OtherActor))
  (set `self.Character` _asbp_side_scroller_character_advanced)
  (`/Game/AdvancedPlatformer/Blueprints/BP_SideScrollerCharacterAdvanced.ResetPowerUpJump` _asbp_side_scroller_character_advanced)
  (`/Engine/EditorBlueprintResources/StandardMacros.DoOnce` false
    (:`Completed`
      (set `/Game/AdvancedPlatformer/Blueprints/BP_SideScrollerCharacterAdvanced.PowerUPJump` true (`self.Character`))
      (`KismetSystemLibrary.PrintString` "Hello" true true (struct :`R` 1.0 :`G` 0.833988 :`B` 0.054318 :`A` 1.0))
      (`ActorComponent.K2_DestroyComponent` (`self.Shape_Cube`))
      (`AudioComponent.Play` (`/Game/AdvancedPlatformer/Blueprints/BP_SideScrollerCharacterAdvanced.PowerUp_Wav` (`self.Character`)) 0.0)
      (bind _returnvalue (`|CreateWidget` "/Game/AdvancedPlatformer/Widgets/BP_PowerUpJump_Widget.BP_PowerUpJump_Widget_C"))
      (`UserWidget.AddToViewport` _returnvalue 0)
      (`KismetSystemLibrary.Delay` 4.0)
      (`self.K2_DestroyActor`))))

(fn `UserConstructionScript`)