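; Speed power-up pickup for the side-scroller character that spins through a rotating movement component added at BeginPlay.
; Box overlap by BP_SideScrollerCharacterAdvanced calls the character's ResetPowerUpSpeed, then a DoOnce sets its PowerUpSpeed flag.
; The same one-shot destroys the cube mesh, plays the character's power-up sound and shows the speed widget.
; The actor destroys itself after a short delay.
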(event `self.ReceiveBeginPlay`
  ;[1 1 1] EventRotatint
  (`AddComponent|NODE_AddRotatingMovementComponent-0`))

(event `self.Box.OnComponentBeginOverlap`
  (params (OverlappedComponent :type "PrimitiveComponent Object Reference") (OtherActor :type "Actor Object Reference") (OtherComp :type "PrimitiveComponent Object Reference") (OtherBodyIndex :type Integer) (bFromSweep :type Boolean) (SweepResult :type "HitResult Structure (by ref)"))
  ;[1 1 1] PowerUpSpeedEvent
  (bind _asbp_side_scroller_character_advanced (cast `/Game/AdvancedPlatformer/Blueprints/BP_SideScrollerCharacterAdvanced` OtherActor))
  (bind _output_get (set `self.Character` _asbp_side_scroller_character_advanced))
  (`/Game/AdvancedPlatformer/Blueprints/BP_SideScrollerCharacterAdvanced.ResetPowerUpSpeed` _output_get)
  (`/Engine/EditorBlueprintResources/StandardMacros.DoOnce` false
    (:`Completed`
      (bind _output_get_2 (set `/Game/AdvancedPlatformer/Blueprints/BP_SideScrollerCharacterAdvanced.PowerUpSpeed` true (`self.Character`)))
      (`KismetSystemLibrary.PrintString` "Hello" _output_get_2 true (struct :`R` 1.0 :`G` 0.833988 :`B` 0.054318 :`A` 1.0))
      (`ActorComponent.K2_DestroyComponent` (`self.Shape_Cube`))
      (`AudioComponent.Play` (`/Game/AdvancedPlatformer/Blueprints/BP_SideScrollerCharacterAdvanced.PowerUp_Wav` (`self.Character`)) 0.0)
      (bind _returnvalue (`|CreateWidget` "/Game/AdvancedPlatformer/Widgets/BP_PowerUpSpeed_Widget.BP_PowerUpSpeed_Widget_C"))
      (`UserWidget.AddToViewport` _returnvalue 0)
      (`KismetSystemLibrary.Delay` 4.0)
      (`self.K2_DestroyActor`))))

(fn `UserConstructionScript`)