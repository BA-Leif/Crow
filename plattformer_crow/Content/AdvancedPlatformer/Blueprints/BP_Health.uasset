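; BP_Health is a health pickup that heals BP_SideScrollerCharacterAdvanced when that character overlaps its Sphere.
; Below 100 health, a DoOnce adds HealthValue without clamping, destroys ShapeSphere and plays the character's HealthWav.
; It then shows BP_Health_Widget for a few seconds before removing it and destroying itself.
; At full health, the pickup is destroyed immediately with no effect.
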(event `self.Sphere.OnComponentBeginOverlap`
  (params (OverlappedComponent :type "PrimitiveComponent Object Reference") (OtherActor :type "Actor Object Reference") (OtherComp :type "PrimitiveComponent Object Reference") (OtherBodyIndex :type Integer) (bFromSweep :type Boolean) (SweepResult :type "HitResult Structure (by ref)"))
  ;[1 1 1] When a player takes a HealthBall, it replenishes his health by an amount equal to the value of a HealthValue. If health is less than 100
  (bind _asbp_side_scroller_character_advanced (cast `/Game/AdvancedPlatformer/Blueprints/BP_SideScrollerCharacterAdvanced` OtherActor))
  (set `self.Character` _asbp_side_scroller_character_advanced)
  (if (< (`/Game/AdvancedPlatformer/Blueprints/BP_SideScrollerCharacterAdvanced.Health` (`self.Character`)) 100.0)
    (`/Engine/EditorBlueprintResources/StandardMacros.DoOnce` false
      (:`Completed`
        (set `/Game/AdvancedPlatformer/Blueprints/BP_SideScrollerCharacterAdvanced.Health` (+ (`/Game/AdvancedPlatformer/Blueprints/BP_SideScrollerCharacterAdvanced.Health` (`self.Character`)) (`self.HealthValue`)) (`self.Character`))
        (`ActorComponent.K2_DestroyComponent` (`self.Shape_Sphere`))
        (`AudioComponent.Play` (`/Game/AdvancedPlatformer/Blueprints/BP_SideScrollerCharacterAdvanced.Health_Wav` (`self.Character`)) 0.0)
        (bind _returnvalue (`|CreateWidget` "/Game/AdvancedPlatformer/Widgets/BP_Health_Widget.BP_Health_Widget_C"))
        (`UserWidget.AddToViewport` _returnvalue 0)
        (`KismetSystemLibrary.Delay` 4.0)
        (`Widget.RemoveFromParent` _returnvalue)
        (`self.K2_DestroyActor`)))
    (else
      (`self.K2_DestroyActor`))))

(fn `UserConstructionScript`)