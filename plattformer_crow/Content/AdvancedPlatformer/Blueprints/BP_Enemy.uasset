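; BP_Enemy is a side-scroller enemy that endlessly patrols between two target points using chained AI Move To calls.
; Touching its capsule destroys the player character, while overlapping its box, meant as a stomp from above, defeats the enemy once.
; Defeat grants XP to the cached player, removes mesh and capsule, plays the player's coin sound and briefly shows an XP widget before destroying the enemy.
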(event `self.ReceiveBeginPlay`
  ;[1 1 1] Event Begin Play
  (bind _asbp_side_scroller_character_advanced (cast `/Game/AdvancedPlatformer/Blueprints/BP_SideScrollerCharacterAdvanced` (`GameplayStatics.GetPlayerCharacter` 0)))
  (set `self.Character` _asbp_side_scroller_character_advanced)
  (`self.Patrol`))

(event `Patrol`
  ;[1 1 1] CustomEventPatrol
  (`|AIMoveTo` self (0.0 0.0 0.0) (`self.TargetPoint`)
    (:`OnSuccess`
      (`|AIMoveTo` self (0.0 0.0 0.0) (`self.TargetPoint2`)
        (:`OnSuccess`
          (`self.Patrol`))))))

(event `self.Capsule.OnComponentBeginOverlap`
  (params (OverlappedComponent :type "PrimitiveComponent Object Reference") (OtherActor :type "Actor Object Reference") (OtherComp :type "PrimitiveComponent Object Reference") (OtherBodyIndex :type Integer) (bFromSweep :type Boolean) (SweepResult :type "HitResult Structure (by ref)"))
  ;[1 1 1] If Enemy Colliding With player, he destroy player
  (bind _asbp_side_scroller_character_advanced (cast `/Game/AdvancedPlatformer/Blueprints/BP_SideScrollerCharacterAdvanced` OtherActor))
  (`self.K2_DestroyActor` _asbp_side_scroller_character_advanced))

(event `self.Box.OnComponentBeginOverlap`
  (params (OverlappedComponent :type "PrimitiveComponent Object Reference") (OtherActor :type "Actor Object Reference") (OtherComp :type "PrimitiveComponent Object Reference") (OtherBodyIndex :type Integer) (bFromSweep :type Boolean) (SweepResult :type "HitResult Structure (by ref)"))
  ;[1 1 1] If a player jumps on top of an enemy, he will destroy the enemy.
  (cast `/Game/AdvancedPlatformer/Blueprints/BP_SideScrollerCharacterAdvanced` OtherActor)
  (`/Engine/EditorBlueprintResources/StandardMacros.DoOnce` false
    (:`Completed`
      (set `/Game/AdvancedPlatformer/Blueprints/BP_SideScrollerCharacterAdvanced.XP` (+ (`/Game/AdvancedPlatformer/Blueprints/BP_SideScrollerCharacterAdvanced.XP` (`self.Character`)) (`self.XPEnemyValue`)) (`self.Character`))
      (`ActorComponent.K2_DestroyComponent` (`self.SK_Mannequin`))
      (`ActorComponent.K2_DestroyComponent` (`self.Capsule`))
      (`AudioComponent.Play` (`/Game/AdvancedPlatformer/Blueprints/BP_SideScrollerCharacterAdvanced.Coin_Wav` (`self.Character`)) 0.0)
      (bind _returnvalue (`|CreateWidget` "/Game/AdvancedPlatformer/Widgets/BP_XPEnemy_Widget.BP_XPEnemy_Widget_C"))
      (`UserWidget.AddToViewport` _returnvalue 0)
      (`KismetSystemLibrary.Delay` 1.0)
      (`Widget.RemoveFromParent` _returnvalue)
      (`self.K2_DestroyActor`))))

(fn `UserConstructionScript`)