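; Checkpoint actor for the advanced side-scroller platformer that saves player progress when an actor tagged Player overlaps it.
; It creates a fresh BP_SaveObject and fills it with the character's location, XP and health, plus a level name converted from its LevelList enum.
; It clears the NewGame flag, overwrites the SaveGame slot, then plays the character's save sound and prints a confirmation.
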(event `self.ReceiveActorBeginOverlap`
  (params (OtherActor :type "Actor Object Reference"))
  ;[1 1 1] When CheckPoint overlap with player, it save player stats
  (if (`self.ActorHasTag` OtherActor "Player")
    (bind _returnvalue (`GameplayStatics.CreateSaveGameObject` "/Game/AdvancedPlatformer/Blueprints/BP_SaveObject.BP_SaveObject_C"))
    (bind _asbp_save_object (cast `/Game/AdvancedPlatformer/Blueprints/BP_SaveObject` _returnvalue))
    (set `self.Save` _asbp_save_object)
    (bind _asbp_side_scroller_character_advanced (cast `/Game/AdvancedPlatformer/Blueprints/BP_SideScrollerCharacterAdvanced` (`GameplayStatics.GetPlayerCharacter` 0)))
    (set `self.Character` _asbp_side_scroller_character_advanced)
    (set `/Game/AdvancedPlatformer/Blueprints/BP_SaveObject.CheckPoint` (`self.K2_GetActorLocation` (`self.Character`)) (`self.Save`))
    (set `/Game/AdvancedPlatformer/Blueprints/BP_SaveObject.XP` (`/Game/AdvancedPlatformer/Blueprints/BP_SideScrollerCharacterAdvanced.XP` (`self.Character`)) (`self.Save`))
    (set `/Game/AdvancedPlatformer/Blueprints/BP_SaveObject.Health` (`/Game/AdvancedPlatformer/Blueprints/BP_SideScrollerCharacterAdvanced.Health` (`self.Character`)) (`self.Save`))
    (set `/Game/AdvancedPlatformer/Blueprints/BP_SaveObject.LevelName` (`KismetStringLibrary.Conv_StringToName` (`|GetEnumeratorNameAsString` (`self.LevelList`))) (`self.Save`))
    (set `/Game/AdvancedPlatformer/Blueprints/BP_SaveObject.NewGame` false (`self.Save`))
    (`GameplayStatics.SaveGameToSlot` (`self.Save`) "SaveGame")
    (`AudioComponent.Play` (`/Game/AdvancedPlatformer/Blueprints/BP_SideScrollerCharacterAdvanced.SaveSound` (`self.Character`)) 0.0)
    (`KismetSystemLibrary.PrintString` "Save")))

(fn `UserConstructionScript`)